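; BP_Axe is an axe actor that shows a fire effect on its head during the player's melee attack.
; On BeginPlay it spawns an inactive torch-fire Niagara system attached to the AxeLow mesh's head socket and caches the player character.
; Each Tick it compares the character's current montage to last frame's, activating the fire for the melee attack montage and deactivating it otherwise.
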(event `self.ReceiveBeginPlay`
  (set `self.Character` (`GameplayStatics.GetPlayerCharacter` 0))
  (bind _returnvalue (`NiagaraFunctionLibrary.SpawnSystemAttached` "/Game/ParticleEffects/NS_TorchFire.NS_TorchFire" (`self.axe_low`) "headSocket" (0.0 0.0 0.0) (struct) "SnapToTargetIncludingScale" false false))
  (set `self.ParticleEffect` _returnvalue))

(event `self.ReceiveTick`
  (params (DeltaSeconds :type "Float (single-precision)"))
  (bind _particleeffect (`self.ParticleEffect`))
  (bind _animmontage (`self.AnimMontage`))
  (set `self.AnimMontage` (`Character.GetCurrentMontage` (`self.Character`)))
  (if (== (`self.AnimMontage`) (`self.LastFrameAnimMontage`))
    _
    (elif (== (`self.AnimMontage`) "/Game/Animations/AM_MeleeAttack.AM_MeleeAttack")
      (`ActorComponent.Activate` _particleeffect false)
      (set `self.LastFrameAnimMontage` _animmontage)
      (else
        (`ActorComponent.Deactivate` _particleeffect)
        (set `self.LastFrameAnimMontage` _animmontage)))))

(fn `UserConstructionScript`)